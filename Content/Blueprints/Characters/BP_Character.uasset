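; Player character Blueprint that handles directional movement, directional attacks and the pause menu through Enhanced Input.
; Each move starts a delayed input cooldown flag, then line-traces the floor to play a grass footstep sound.
; Attacks chain advance and retreat timelines into AnimateAttack, blocking re-triggering until both finish.
; Pause shows WBP_PlayerPause, switching input mode and cursor; its callbacks resume play or raise the return-to-main-menu game event.
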(event Custom|Resume%20Game%20Event%20Listener
  (Widget|RemovefromParent (Variables|Default|GetPause%20menu))
  (Variables|/Script/Engine.PlayerController|SetbShowMouseCursor (Game|GetPlayerController 0) false)
  (Variables|Default|SetOn%20Pause false)
  (Input|SetInputModeGameOnly (Game|GetPlayerController 0) false))

(event Custom|Return%20to%20Main%20Menu%20Event%20Listener
  (Input|SetInputModeGameandUI (Game|GetPlayerController 0) 0 "DoNotLock" true false)
  (Widget|RemovefromParent (Variables|Default|GetPause%20menu))
  (Variables|Default|SetOn%20Pause false)
  (Default|CallOnReturntoMainMenu (Variables|Default|GetgameEvents)))

(event Input|EnhancedActionEvents|EnhancedInputActionIA_MoveUp
  (params (ActionValue :type Boolean) (ElapsedSeconds :type Float%20%28double-precision%29) (TriggeredSeconds :type Float%20%28double-precision%29) (InputAction :type Input%20Action%20Object%20Reference :default "/Game/Blueprints/Inputs/IA_MoveUp.IA_MoveUp"))
  (bind _returnvalue (Transformation|GetActorLocation))
  ;[1 1 1] Player Movement
  (:Started
    (Class|LRPlayerCharacter|MoveUp)
    (Variables|Default|SetplayerCanReceiveMovementInput false)
    (Utilities|FlowControl|Delay (Variables|Default|GetmovementDelayTime))
    (Variables|Default|SetplayerCanReceiveMovementInput true)
    (bind (_outhit _returnvalue_2) (Collision|LineTraceByChannel _returnvalue (+ _returnvalue (Math|Vector|NegateVector (* (Transformation|GetActorUpVector) (Variables|Default|GetfloorDetectionRaySize)))) "TraceTypeQuery1" false 0 "ForDuration" true "(R=0.000000,G=0.260827,B=1.000000,A=1.000000)"))
    (if _returnvalue_2
      (switch Utilities|FlowControl|Switch|SwitchonEPhysicalSurface (Variables|/Script/PhysicsCore.PhysicalMaterial|GetSurfaceType (.PhysMat (Collision|BreakHitResult _outhit)))
        (:SurfaceType_Default
          _)
        (:SurfaceType1
          _))
      (Audio|PlaySound2D "/Game/Sound/SFX/SC_GrassFootstep.SC_GrassFootstep" 1.0 1.0 0.0 0 0))))

(event Input|EnhancedActionEvents|EnhancedInputActionIA_MoveDown
  (params (ActionValue :type Boolean) (ElapsedSeconds :type Float%20%28double-precision%29) (TriggeredSeconds :type Float%20%28double-precision%29) (InputAction :type Input%20Action%20Object%20Reference :default "/Game/Blueprints/Inputs/IA_MoveDown.IA_MoveDown"))
  (bind _returnvalue (Transformation|GetActorLocation))
  ;[1 1 1] Player Movement
  (:Started
    (Class|LRPlayerCharacter|MoveDown)
    (Variables|Default|SetplayerCanReceiveMovementInput false)
    (Utilities|FlowControl|Delay (Variables|Default|GetmovementDelayTime))
    (Variables|Default|SetplayerCanReceiveMovementInput true)
    (bind (_outhit _returnvalue_2) (Collision|LineTraceByChannel _returnvalue (+ _returnvalue (Math|Vector|NegateVector (* (Transformation|GetActorUpVector) (Variables|Default|GetfloorDetectionRaySize)))) "TraceTypeQuery1" false 0 "ForDuration" true "(R=0.000000,G=0.260827,B=1.000000,A=1.000000)"))
    (if _returnvalue_2
      (switch Utilities|FlowControl|Switch|SwitchonEPhysicalSurface (Variables|/Script/PhysicsCore.PhysicalMaterial|GetSurfaceType (.PhysMat (Collision|BreakHitResult _outhit)))
        (:SurfaceType_Default
          _)
        (:SurfaceType1
          _))
      (Audio|PlaySound2D "/Game/Sound/SFX/SC_GrassFootstep.SC_GrassFootstep" 1.0 1.0 0.0 0 0))))

(event Input|EnhancedActionEvents|EnhancedInputActionIA_MoveRight
  (params (ActionValue :type Boolean) (ElapsedSeconds :type Float%20%28double-precision%29) (TriggeredSeconds :type Float%20%28double-precision%29) (InputAction :type Input%20Action%20Object%20Reference :default "/Game/Blueprints/Inputs/IA_MoveRight.IA_MoveRight"))
  (bind _returnvalue (Transformation|GetActorLocation))
  ;[1 1 1] Player Movement
  (:Started
    (Class|LRPlayerCharacter|MoveRight)
    (Variables|Default|SetplayerCanReceiveMovementInput false)
    (Utilities|FlowControl|Delay (Variables|Default|GetmovementDelayTime))
    (Variables|Default|SetplayerCanReceiveMovementInput true)
    (bind (_outhit _returnvalue_2) (Collision|LineTraceByChannel _returnvalue (+ _returnvalue (Math|Vector|NegateVector (* (Transformation|GetActorUpVector) (Variables|Default|GetfloorDetectionRaySize)))) "TraceTypeQuery1" false 0 "ForDuration" true "(R=0.000000,G=0.260827,B=1.000000,A=1.000000)"))
    (if _returnvalue_2
      (switch Utilities|FlowControl|Switch|SwitchonEPhysicalSurface (Variables|/Script/PhysicsCore.PhysicalMaterial|GetSurfaceType (.PhysMat (Collision|BreakHitResult _outhit)))
        (:SurfaceType_Default
          _)
        (:SurfaceType1
          _))
      (Audio|PlaySound2D "/Game/Sound/SFX/SC_GrassFootstep.SC_GrassFootstep" 1.0 1.0 0.0 0 0))))

(event Input|EnhancedActionEvents|EnhancedInputActionIA_MoveLeft
  (params (ActionValue :type Boolean) (ElapsedSeconds :type Float%20%28double-precision%29) (TriggeredSeconds :type Float%20%28double-precision%29) (InputAction :type Input%20Action%20Object%20Reference :default "/Game/Blueprints/Inputs/IA_MoveLeft.IA_MoveLeft"))
  (bind _returnvalue (Transformation|GetActorLocation))
  ;[1 1 1] Player Movement
  (:Started
    (Class|LRPlayerCharacter|MoveLeft)
    (Variables|Default|SetplayerCanReceiveMovementInput false)
    (Utilities|FlowControl|Delay (Variables|Default|GetmovementDelayTime))
    (Variables|Default|SetplayerCanReceiveMovementInput true)
    (bind (_outhit _returnvalue_2) (Collision|LineTraceByChannel _returnvalue (+ _returnvalue (Math|Vector|NegateVector (* (Transformation|GetActorUpVector) (Variables|Default|GetfloorDetectionRaySize)))) "TraceTypeQuery1" false 0 "ForDuration" true "(R=0.000000,G=0.260827,B=1.000000,A=1.000000)"))
    (if _returnvalue_2
      (switch Utilities|FlowControl|Switch|SwitchonEPhysicalSurface (Variables|/Script/PhysicsCore.PhysicalMaterial|GetSurfaceType (.PhysMat (Collision|BreakHitResult _outhit)))
        (:SurfaceType_Default
          _)
        (:SurfaceType1
          _))
      (Audio|PlaySound2D "/Game/Sound/SFX/SC_GrassFootstep.SC_GrassFootstep" 1.0 1.0 0.0 0 0))))

(event Input|EnhancedActionEvents|EnhancedInputActionIA_AttackUp
  (params (ActionValue :type Boolean) (ElapsedSeconds :type Float%20%28double-precision%29) (TriggeredSeconds :type Float%20%28double-precision%29) (InputAction :type Input%20Action%20Object%20Reference :default "/Game/Blueprints/Inputs/IA_AttackUp.IA_AttackUp"))
  ;[1 1 1] Player Attack
  (:Started
    (Class|LRPlayerCharacter|AttackUp)
    (if (Variables|Default|GetplayerCanReceiveAttackInput)
      (Variables|Default|SetplayerCanReceiveAttackInput false)
      (bind _foward (Timeline|Advence%20Attack%20Animation PlayFromStart)
        (:Update
          (Class|LRPlayerCharacter|AnimateAttack _foward))
        (:Finished
          (bind _backward (Timeline|Retriet%20Attack%20Animation PlayFromStart)
            (:Update
              (Class|LRPlayerCharacter|AnimateAttack _backward))
            (:Finished
              (Variables|Default|SetplayerCanReceiveAttackInput true))))))))

(event Input|EnhancedActionEvents|EnhancedInputActionIA_AttackDown
  (params (ActionValue :type Boolean) (ElapsedSeconds :type Float%20%28double-precision%29) (TriggeredSeconds :type Float%20%28double-precision%29) (InputAction :type Input%20Action%20Object%20Reference :default "/Game/Blueprints/Inputs/IA_AttackDown.IA_AttackDown"))
  ;[1 1 1] Player Attack
  (:Started
    (Class|LRPlayerCharacter|AttackDown)
    (if (Variables|Default|GetplayerCanReceiveAttackInput)
      (Variables|Default|SetplayerCanReceiveAttackInput false)
      (bind _foward (Timeline|Advence%20Attack%20Animation PlayFromStart)
        (:Update
          (Class|LRPlayerCharacter|AnimateAttack _foward))
        (:Finished
          (bind _backward (Timeline|Retriet%20Attack%20Animation PlayFromStart)
            (:Update
              (Class|LRPlayerCharacter|AnimateAttack _backward))
            (:Finished
              (Variables|Default|SetplayerCanReceiveAttackInput true))))))))

(event Input|EnhancedActionEvents|EnhancedInputActionIA_AttackLeft
  (params (ActionValue :type Boolean) (ElapsedSeconds :type Float%20%28double-precision%29) (TriggeredSeconds :type Float%20%28double-precision%29) (InputAction :type Input%20Action%20Object%20Reference :default "/Game/Blueprints/Inputs/IA_AttackLeft.IA_AttackLeft"))
  ;[1 1 1] Player Attack
  (:Started
    (Class|LRPlayerCharacter|AttackLeft)
    (if (Variables|Default|GetplayerCanReceiveAttackInput)
      (Variables|Default|SetplayerCanReceiveAttackInput false)
      (bind _foward (Timeline|Advence%20Attack%20Animation PlayFromStart)
        (:Update
          (Class|LRPlayerCharacter|AnimateAttack _foward))
        (:Finished
          (bind _backward (Timeline|Retriet%20Attack%20Animation PlayFromStart)
            (:Update
              (Class|LRPlayerCharacter|AnimateAttack _backward))
            (:Finished
              (Variables|Default|SetplayerCanReceiveAttackInput true))))))))

(event Input|EnhancedActionEvents|EnhancedInputActionIA_AttackRight
  (params (ActionValue :type Boolean) (ElapsedSeconds :type Float%20%28double-precision%29) (TriggeredSeconds :type Float%20%28double-precision%29) (InputAction :type Input%20Action%20Object%20Reference :default "/Game/Blueprints/Inputs/IA_AttackRight.IA_AttackRight"))
  ;[1 1 1] Player Attack
  (:Started
    (Class|LRPlayerCharacter|AttackRight)
    (if (Variables|Default|GetplayerCanReceiveAttackInput)
      (Variables|Default|SetplayerCanReceiveAttackInput false)
      (bind _foward (Timeline|Advence%20Attack%20Animation PlayFromStart)
        (:Update
          (Class|LRPlayerCharacter|AnimateAttack _foward))
        (:Finished
          (bind _backward (Timeline|Retriet%20Attack%20Animation PlayFromStart)
            (:Update
              (Class|LRPlayerCharacter|AnimateAttack _backward))
            (:Finished
              (Variables|Default|SetplayerCanReceiveAttackInput true))))))))

(event Input|EnhancedActionEvents|EnhancedInputActionIA_Pause
  (params (ActionValue :type Boolean) (ElapsedSeconds :type Float%20%28double-precision%29) (TriggeredSeconds :type Float%20%28double-precision%29) (InputAction :type Input%20Action%20Object%20Reference :default "/Game/Blueprints/Inputs/IA_Pause.IA_Pause"))
  ;[1 1 1] Pause
  (:Started
    (if (not (Variables|Default|GetOn%20Pause))
      (UserInterface|Viewport|AddtoViewport (Variables|Default|GetPause%20menu) 0)
      (Input|SetInputModeUIOnly (Game|GetPlayerController 0) (Variables|Default|GetPause%20menu) "DoNotLock" false)
      (Variables|/Script/Engine.PlayerController|SetbShowMouseCursor (Game|GetPlayerController 0) true)
      (Variables|Default|SetOn%20Pause true))))

(event EventBeginPlay
  (|CallParentFunction)
  (bind _returnvalue (UserInterface|CreateWidget "/Game/Blueprints/UI/WBP_PlayerPause.WBP_PlayerPause_C"))
  (bind _output_get (Variables|Default|SetPause%20menu _returnvalue))
  (EventDispatchers|BindEventtoOnResumeGame _output_get (EventDispatchers|CreateEvent :!event Custom|Resume%20Game%20Event%20Listener))
  (EventDispatchers|BindEventtoOnReturntoMainMenu (Variables|Default|GetPause%20menu) (EventDispatchers|CreateEvent :!event Custom|Return%20to%20Main%20Menu%20Event%20Listener)))

(fn ConstructionScript)